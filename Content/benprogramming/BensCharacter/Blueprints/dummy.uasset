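; Target dummy character that can be locked on to, takes damage and plays hit-react or death animations.
; TargetLockon toggles the visibility of its TargetVisual marker on alternate calls.
; AnyDamage subtracts Health behind a DoOnce gate that reopens shortly after a hit react but stays closed after death, blocking further damage.
; A helper function returns the distance to the player character.
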(event `/Game/benprogramming/BensCharacter/Blueprints/Game_BP.TargetLockOn`
  (bind _targetvisual (`self.targetVisual`))
  (`/Engine/EditorBlueprintResources/StandardMacros.FlipFlop`
    (:`A`
      (`SceneComponent.SetHiddenInGame` _targetvisual false false))
    (:`B`
      (`SceneComponent.SetHiddenInGame` _targetvisual true false))))

(event `self.ReceiveAnyDamage`
  (params (Damage :type "Float (single-precision)") (DamageType :type "DamageType Object Reference") (InstigatedBy :type "Controller Object Reference") (DamageCauser :type "Actor Object Reference"))
  (`/Engine/EditorBlueprintResources/StandardMacros.DoOnce` false :!label _label
    (:`Completed`
      (bind _output_get (set `self.health` (- (`self.health`) Damage)))
      (if (<= _output_get 0.0)
        (`self.PlayAnimMontage` "/Game/benprogramming/animations/Death_Montage.Death_Montage")
        (else
          (`self.PlayAnimMontage` "/Game/benprogramming/animations/HitReact_Montage.HitReact_Montage")
          (`KismetSystemLibrary.Delay` 0.2)
          (goto _label :!via `Reset`))))))

(fn `DistanceFromPlayercheck`
  (returns (Distancefromplayer :type "Float (double-precision)"))
  (return (`self.GetDistanceTo` (`GameplayStatics.GetPlayerCharacter` 0))))

(fn `UserConstructionScript`)